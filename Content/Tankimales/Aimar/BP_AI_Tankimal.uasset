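; AI-controlled Tankimal opponent character whose defeat triggers the player's win.
; Shortly after BeginPlay it initializes its life HUD through the life component.
; Receivedamage plays the visual component's damage animation, removes a life, then plays a hurt sound while lives remain.
; At zero lives it marks itself dead, plays the death sound, disables capsule collision, freezes player input and plays the player Tankimal's win sound.
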(event `self.ReceiveBeginPlay`
  (`KismetSystemLibrary.Delay` 0.1)
  (`/Game/Tankimales/Fran/BP_LifeComponent.InitHUD` (`self.BP_LifeComponent`) 1))

(fn `Receivedamage`
  (bind _returnvalue (`GameplayStatics.GetPlayerCharacter` 0))
  (bind _bpc_visualcharacter (`self.BPC_VisualCharacter`))
  (`/Game/Tankimales/Eva/BPC_VisualCharacter.ReceiveDamageAnim` (`self.BPC_VisualCharacter`))
  (`/Game/Tankimales/Fran/BP_LifeComponent.RemoveLife` (`self.BP_LifeComponent`))
  (bind _currentlives (`/Game/Tankimales/Fran/BP_LifeComponent.GetCurrentLives` (`self.BP_LifeComponent`)))
  (if (== _currentlives 0)
    (set `self.Dead` true)
    (`GameplayStatics.PlaySound2D` (`/Game/Tankimales/Eva/BPC_VisualCharacter.Sound_Death` _bpc_visualcharacter) 1.0 1.0 0.0 null null)
    (`PrimitiveComponent.SetCollisionEnabled` (`self.CapsuleComponent`) "NoCollision")
    (`self.DisableInput` _returnvalue (`GameplayStatics.GetPlayerController` 0))
    (bind _asbp_tankimal (cast `/Game/Tankimales/BP_Tankimal` _returnvalue))
    (`GameplayStatics.PlaySound2D` (`/Game/Tankimales/Eva/BPC_VisualCharacter.Sound_Win` (`/Game/Tankimales/BP_Tankimal.BPC_VisualCharacter` _asbp_tankimal)) 1.0 1.0 0.0 null null)
    (else
      (`GameplayStatics.PlaySound2D` (`/Game/Tankimales/Eva/BPC_VisualCharacter.Sound_Hurt` _bpc_visualcharacter) 1.0 1.0 0.0 null null))))

(fn `UserConstructionScript`)