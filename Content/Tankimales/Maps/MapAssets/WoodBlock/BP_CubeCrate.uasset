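; BP_CubeCrate is a destructible crate map asset in Tankimales that breaks after a set number of hits.
; Each ReceiveDamage event takes one from Lifes and spawns an actor at the crate's transform.
; On the hit that brings Lifes to zero, that spawn has Pooof enabled, a 2D explosion sound plays, and the crate destroys itself after a short delay.
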(event `ReceiveDamage`
  (set `self.Lifes` (- (`self.Lifes`) 1))
  (if (== (`self.Lifes`) 0)
    (`|SpawnActorFromClass` "/Game/CBLaP/Textures/BP_ComicMessage.BP_ComicMessage_C" (`self.GetTransform`) "Undefined" "MultiplyWithRoot" null false true null)
    (`GameplayStatics.PlaySound2D` "/Game/Tankimales/Eva/Sounds/402006__eardeer__explosion_high_to_low_1.402006__eardeer__explosion_high_to_low_1" 0.5 1.0 0.0 null null)
    (`KismetSystemLibrary.Delay` 0.2)
    (`self.K2_DestroyActor`)
    (else
      (`|SpawnActorFromClass` "/Game/CBLaP/Textures/BP_ComicMessage.BP_ComicMessage_C" (`self.GetTransform`) "Undefined" "MultiplyWithRoot" null false false null))))

(fn `UserConstructionScript`)