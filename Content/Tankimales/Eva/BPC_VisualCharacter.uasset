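; Visual component that sets the look and sounds of a Tankimals character for Flamingo, Frog, Bee or Red Panda.
; ChangeCharacter swaps the owner's skeletal mesh and anim class, then stores that animal's damage montage and shoot, win, death and hurt sounds.
; ReceiveDamageAnim plays the stored damage montage on the owning Character.
; ShootAnim always plays the Flamingo shoot montage, whichever animal is selected.
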(fn `ChangeCharacter`
  (params (Character :type "/Game/Tankimales/Fran/E_Characters Enum" :default "NewEnumerator0"))
  (bind _ascharacter (cast `Character` (`self.GetOwner`)))
  (switch `/Game/Tankimales/Fran/E_Characters` Character
    (:`NewEnumerator0`
      (bind _mesh (`Character.Mesh` _ascharacter))
      (`SkeletalMeshComponent.SetSkeletalMeshAsset` _mesh "/Game/Tankimales/Eva/Characters/Flamingo/Mech_FernandoTheFlamingo.Mech_FernandoTheFlamingo")
      (`SkeletalMeshComponent.SetAnimInstanceClass` _mesh "/Game/Tankimales/Eva/BPA_Tankimal.BPA_Tankimal_C")
      (set `self.Anim_Damaged` "/Game/Tankimales/Eva/Characters/Flamingo/Animations/Flamingo_Damaged.Flamingo_Damaged")
      (set `self.Sound_Shoot` "/Game/Tankimales/Eva/Sounds/Shoot/472095__claymorexx__08-disparo2.472095__claymorexx__08-disparo2")
      (set `self.Sound_Win` "/Game/Tankimales/Eva/Sounds/Laugh/218869__robinhood76__04840-mad-man-laughter-dry.218869__robinhood76__04840-mad-man-laughter-dry")
      (set `self.Sound_Death` "/Game/Tankimales/Eva/Sounds/Death/345456__artmasterrich__male_death_04.345456__artmasterrich__male_death_04")
      (set `self.Sound_Hurt` "/Game/Tankimales/Eva/Sounds/Hurt/345436__artmasterrich__male_hurt_04.345436__artmasterrich__male_hurt_04"))
    (:`NewEnumerator1`
      (`SkeletalMeshComponent.SetSkeletalMeshAsset` _mesh "/Game/Tankimales/Eva/Characters/Frog/Mech_FinnTheFrog.Mech_FinnTheFrog")
      (`SkeletalMeshComponent.SetAnimInstanceClass` _mesh "/Game/Tankimales/Eva/Characters/Frog/BPA_Frog.BPA_Frog_C")
      (set `self.Anim_Damaged` "/Game/Tankimales/Eva/Characters/Frog/Frog_Damaged.Frog_Damaged")
      (set `self.Sound_Shoot` "/Game/Tankimales/Eva/Sounds/Shoot/disparoGirl.disparoGirl")
      (set `self.Sound_Win` "/Game/Tankimales/Eva/Sounds/Laugh/84746__robinhood76__01385-witch-cackle-3-natural.84746__robinhood76__01385-witch-cackle-3-natural")
      (set `self.Sound_Death` "/Game/Tankimales/Eva/Sounds/Death/345466__artmasterrich__male_nooo_02.345466__artmasterrich__male_nooo_02")
      (set `self.Sound_Hurt` "/Game/Tankimales/Eva/Sounds/Hurt/345438__artmasterrich__male_hurt_02.345438__artmasterrich__male_hurt_02"))
    (:`NewEnumerator2`
      (`SkeletalMeshComponent.SetSkeletalMeshAsset` _mesh "/Game/Tankimales/Eva/Characters/Bee/Mech_BarbaraTheBee.Mech_BarbaraTheBee")
      (`SkeletalMeshComponent.SetAnimInstanceClass` _mesh "/Game/Tankimales/Eva/Characters/Bee/BPA_Bee.BPA_Bee_C")
      (set `self.Anim_Damaged` "/Game/Tankimales/Eva/Characters/Bee/Bee_Damaged.Bee_Damaged")
      (set `self.Sound_Shoot` "/Game/Tankimales/Eva/Sounds/Shoot/365637__obxjohn__pew-pew-two.365637__obxjohn__pew-pew-two")
      (set `self.Sound_Win` "/Game/Tankimales/Eva/Sounds/Laugh/360733__robinhood76__06862-silly-cartoon-kid-laughter.360733__robinhood76__06862-silly-cartoon-kid-laughter")
      (set `self.Sound_Death` "/Game/Tankimales/Eva/Sounds/Death/345463__artmasterrich__male_nooo_01.345463__artmasterrich__male_nooo_01")
      (set `self.Sound_Hurt` "/Game/Tankimales/Eva/Sounds/Hurt/345433__artmasterrich__male_hurt_01.345433__artmasterrich__male_hurt_01"))
    (:`NewEnumerator3`
      (`SkeletalMeshComponent.SetSkeletalMeshAsset` _mesh "/Game/Tankimales/Eva/Characters/Fox/Mech_RaeTheRedPanda.Mech_RaeTheRedPanda")
      (`SkeletalMeshComponent.SetAnimInstanceClass` _mesh "/Game/Tankimales/Eva/Characters/Fox/BPA_RedPanda.BPA_RedPanda_C")
      (set `self.Anim_Damaged` "/Game/Tankimales/Eva/Characters/Fox/RedPanda_Damaged.RedPanda_Damaged")
      (set `self.Sound_Shoot` "/Game/Tankimales/Eva/Sounds/Shoot/472096__claymorexx__07-disparo1.472096__claymorexx__07-disparo1")
      (set `self.Sound_Win` "/Game/Tankimales/Eva/Sounds/Laugh/591303__robinhood76__10505-male-tricky-laughter.591303__robinhood76__10505-male-tricky-laughter")
      (set `self.Sound_Death` "/Game/Tankimales/Eva/Sounds/Death/345450__artmasterrich__male_death_03.345450__artmasterrich__male_death_03")
      (set `self.Sound_Hurt` "/Game/Tankimales/Eva/Sounds/Hurt/345439__artmasterrich__male_hurt_03.345439__artmasterrich__male_hurt_03"))))

(fn `ReceiveDamageAnim`
  (bind _ascharacter (cast `Character` (`self.GetOwner`)))
  (`Character.PlayAnimMontage` _ascharacter (`self.Anim_Damaged`) 1.0 "None"))

(fn `ShootAnim`
  (bind _ascharacter (cast `Character` (`self.GetOwner`)))
  (`Character.PlayAnimMontage` _ascharacter "/Game/Tankimales/Eva/Characters/Flamingo/Animations/Flamingo_Shoot.Flamingo_Shoot" 1.0 "None"))