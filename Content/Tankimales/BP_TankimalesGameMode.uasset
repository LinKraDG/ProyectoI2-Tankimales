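; Game mode for Tankimales that overrides ChoosePlayerStart to give each of two local players a designated spawn point.
; It maps player controller 0 to the tag PlayerStart1 and controller 1 to PlayerStart2.
; It then searches all PlayerStart actors and returns the first with a matching tag, or none if no tag matches.
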(fn `ChoosePlayerStart`
  (params (Player :type "Controller Object Reference"))
  (returns (ReturnValue :type "Actor Object Reference"))
  (locals (PlayerStartTag :type String))
  (if (== Player (`GameplayStatics.GetPlayerController` 0))
    (set `local.PlayerStartTag` "PlayerStart1")
    (elif (== Player (`GameplayStatics.GetPlayerController` 1))
      (set `local.PlayerStartTag` "PlayerStart2")))
  (bind _outactors (`GameplayStatics.GetAllActorsOfClass` "/Script/Engine.PlayerStart"))
  (for _array_element _outactors
    (if (== (`PlayerStart.PlayerStartTag` _array_element) (`local.PlayerStartTag`))
      (return _array_element)))
  (return null))

(fn `UserConstructionScript`)