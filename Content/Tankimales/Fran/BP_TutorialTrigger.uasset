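; BP_TutorialTrigger is a one-shot pickup-style trigger that shows a tutorial message when a player Tankimal enters it.
; On Box overlap by a BP_Tankimal, it passes its TitleToShow, TextToShow and that tank to BP_TankimalesHUD's ShowTutorial, then destroys itself.
; Tick spins the static mesh around its yaw axis by a fixed step per frame, independent of delta time.
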(event `self.ReceiveBeginPlay`
  (add `PrimitiveComponent.OnComponentBeginOverlap` (`self.Box`) (delegate `OnComponentBeginOverlap_Event`)))

(event `OnComponentBeginOverlap_Event`
  (params (OverlappedComponent :type "PrimitiveComponent Object Reference") (OtherActor :type "Actor Object Reference") (OtherComp :type "PrimitiveComponent Object Reference") (OtherBodyIndex :type Integer) (bFromSweep :type Boolean) (SweepResult :type "HitResult Structure (by ref)"))
  (bind _asbp_tankimal (cast `/Game/Tankimales/BP_Tankimal` OtherActor))
  (bind _asbp_tankimales_hud (cast `/Game/UI/BP_TankimalesHUD` (`PlayerController.GetHUD` (`GameplayStatics.GetPlayerController` 0))))
  (`/Game/UI/BP_TankimalesHUD.ShowTutorial` _asbp_tankimales_hud (`self.TextToShow`) (`self.TitleToShow`) _asbp_tankimal)
  (`self.K2_DestroyActor` self))

(event `self.ReceiveTick`
  (params (DeltaSeconds :type "Float (single-precision)"))
  (bind _staticmesh (`self.StaticMesh`))
  (`SceneComponent.K2_SetRelativeRotation` _staticmesh (`KismetMathLibrary.MakeRotator` (.roll (`SceneComponent.RelativeRotation` _staticmesh)) (.pitch (`SceneComponent.RelativeRotation` _staticmesh)) (+ (.yaw (`SceneComponent.RelativeRotation` _staticmesh)) 1.0)) false false))

(fn `UserConstructionScript`)