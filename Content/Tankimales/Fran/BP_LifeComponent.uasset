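; BP_LifeComponent tracks a Tankimales player's lives and reports them to the HUD.
; InitHUD stores the player index, gets the UI reference from player controller 0's BP_TankimalesHUD, and initializes that player's display.
; RemoveLife and AddLife step the count within zero and MaxLives, pushing each change to the UI through UpdateHUD.
; GetCurrentLives exposes the current count.
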(fn `AddLife`
  (if (< (`self.CurrentLives`) (`self.MaxLives`))
    (set `self.CurrentLives` (+ (`self.CurrentLives`) 1))
    (`self.UpdateHUD`)))

(fn `GetCurrentLives`
  (returns (CurrentLives :type Integer))
  (return (`self.CurrentLives`)))

(fn `InitHUD`
  (params (PlayerIndex :type Integer))
  (set `self.PlayerIndex` PlayerIndex)
  (bind _asbp_tankimales_hud (cast `/Game/UI/BP_TankimalesHUD` (`PlayerController.GetHUD` (`GameplayStatics.GetPlayerController` 0))))
  (bind _ui_ref (`/Game/UI/BP_TankimalesHUD.UI_Ref` _asbp_tankimales_hud))
  (set `self.HudUIRef` _ui_ref)
  (`/Game/UI/WB_HUDUI.InitPlayer` _ui_ref (`self.PlayerIndex`))
  (`self.UpdateHUD`))

(fn `RemoveLife`
  (if (> (`self.CurrentLives`) 0)
    (set `self.CurrentLives` (- (`self.CurrentLives`) 1))
    (`self.UpdateHUD`)))

(fn `UpdateHUD`
  (bind _huduiref (`self.HudUIRef`))
  (`/Engine/EditorBlueprintResources/StandardMacros.IsValid` _huduiref
    (:`Is Valid`
      (`/Game/UI/WB_HUDUI.UpdatePlayerLives` _huduiref (`self.CurrentLives`) (`self.PlayerIndex`)))))