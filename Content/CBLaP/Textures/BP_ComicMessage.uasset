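; BP_ComicMessage is a short-lived comic-style pop-up message actor that appears, grows and vanishes.
; On BeginPlay it picks its material from the Ugh and Pooof flags, or randomly from a Materials array, and randomizes the texture's yaw and height.
; A delay loop enlarges the texture in small steps until it passes a randomly re-rolled limit, then the actor briefly holds and destroys itself.
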(event `self.ReceiveBeginPlay`
  (bind _scale (`self.Scale`))
  (bind _texture (`self.Texture`))
  (if (`self.Ugh`)
    (`PrimitiveComponent.SetMaterial` (`self.Texture`) 0 "/Game/CBLaP/Textures/MI_Ugh.MI_Ugh")
    (elif (`self.Pooof`)
      (`PrimitiveComponent.SetMaterial` (`self.Texture`) 0 "/Game/CBLaP/Textures/MI_Pooof.MI_Pooof")
      (else
        (`PrimitiveComponent.SetMaterial` (`self.Texture`) 0 (`KismetArrayLibrary.Array_Random` (`self.Materials`))))))
  (`SceneComponent.K2_SetWorldRotation` _texture (`KismetMathLibrary.MakeRotator` 0.0 0.0 (`KismetMathLibrary.RandomFloatInRange` 70.0 110.0)) false false)
  (`SceneComponent.K2_SetRelativeLocation` _texture (`KismetMathLibrary.MakeVector` 0.0 0.0 (`KismetMathLibrary.RandomFloatInRange` 120.0 140.0)) false false)
  (if (<= (`self.Scale`) (`KismetMathLibrary.RandomFloatInRange` 3.0 4.5)) :!label _label
    (`SceneComponent.SetWorldScale3D` (`self.Texture`) (`KismetMathLibrary.MakeVector` _scale _scale _scale))
    (`KismetSystemLibrary.Delay` 0.03)
    (set `self.Scale` (+ (`self.Scale`) 0.5))
    (goto _label)
    (else
      (`KismetSystemLibrary.Delay` 0.2)
      (`self.K2_DestroyActor`))))

(fn `UserConstructionScript`)